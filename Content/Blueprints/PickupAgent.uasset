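; Pickup component that lets its owner grab, carry and drop physics Pickup objects.
; Tick line-traces from the owner's camera and marks the targeted Pickup through custom depth stencil.
; Grabbing disables gravity and raises damping, so a force pulls the object toward a point ahead of the camera.
; Toggling again or a time-shift event restores physics, zeroes velocity and reports the drop location through the object's OnEquivalentMoved.
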(event Custom|Toggle%20Pickup
  (bind _linetracedobject (Variables|Default|GetLineTracedObject))
  (Utilities|IsValid (Variables|Default|GetHeldObject) ; If object is held
    (:Is%20Valid
      (Default|SetGravityEnabled (Variables|Default|GetHeldObject) true)
      (Class|PrimitiveComponent|SetLinearDamping (Variables|/Game/Blueprints/Pickup.Pickup_C|GetGeometry (Variables|Default|GetHeldObject)) 0.01)
      (Class|PrimitiveComponent|SetAngularDamping (Variables|/Game/Blueprints/Pickup.Pickup_C|GetGeometry (Variables|Default|GetHeldObject)) 0.0)
      (Physics|SetPhysicsLinearVelocity (Variables|/Game/Blueprints/Pickup.Pickup_C|GetGeometry (Variables|Default|GetHeldObject)) "0, 0, 0" false "None")
      (Default|OnEquivalentMoved (Variables|Default|GetHeldObject) (Transformation|GetWorldLocation (Variables|/Game/Blueprints/Pickup.Pickup_C|GetGeometry (Variables|Default|GetHeldObject))))
      (Variables|Default|SetHeldObject 0))
    (:Is%20Not%20Valid
      (Utilities|IsValid _linetracedobject ; If looking at object
        (:Is%20Valid
          (Default|SetGravityEnabled _linetracedobject false)
          (bind _output_get (Variables|Default|SetHeldObject _linetracedobject))
          (Class|PrimitiveComponent|SetLinearDamping (Variables|/Game/Blueprints/Pickup.Pickup_C|GetGeometry _output_get) 15.0)
          (Class|PrimitiveComponent|SetAngularDamping (Variables|/Game/Blueprints/Pickup.Pickup_C|GetGeometry _output_get) 1.5e+02))))))

(event Custom|On%20Time%20Shifter
  (Utilities|IsValid (Variables|Default|GetHeldObject) ; If object is held
    (:Is%20Valid
      (Default|SetGravityEnabled (Variables|Default|GetHeldObject) true)
      (Class|PrimitiveComponent|SetLinearDamping (Variables|/Game/Blueprints/Pickup.Pickup_C|GetGeometry (Variables|Default|GetHeldObject)) 0.01)
      (Class|PrimitiveComponent|SetAngularDamping (Variables|/Game/Blueprints/Pickup.Pickup_C|GetGeometry (Variables|Default|GetHeldObject)) 0.0)
      (Physics|SetPhysicsLinearVelocity (Variables|/Game/Blueprints/Pickup.Pickup_C|GetGeometry (Variables|Default|GetHeldObject)) "0, 0, 0" false "None")
      (Default|OnEquivalentMoved (Variables|Default|GetHeldObject) (Transformation|GetWorldLocation (Variables|/Game/Blueprints/Pickup.Pickup_C|GetGeometry (Variables|Default|GetHeldObject))))
      (Variables|Default|SetHeldObject 0))))

(event EventBeginPlay)

(event EventTick
  (params (DeltaSeconds :type Float%20%28single-precision%29))
  (bind _returnvalue (Components|GetOwner))
  (bind _returnvalue_2 (Components|GetOwner))
  (bind _returnvalue_3 (|GetTargetPosition))
  (bind _heldobject (Variables|Default|GetHeldObject))
  (bind _returnvalue_4 (Actor|GetComponentbyClass _returnvalue_2 "/Script/Engine.CameraComponent"))
  (bind _returnvalue_5 (Actor|GetComponentbyClass _heldobject "/Script/Engine.PrimitiveComponent"))
  (bind _returnvalue_6 (Actor|GetComponentbyClass _returnvalue "/Script/Engine.CameraComponent"))
  (bind _returnvalue_7 (Math|Vector|GetForwardVector _returnvalue_6))
  (bind _returnvalue_8 (Transformation|GetWorldLocation _returnvalue_4))
  (Utilities|IsValid (Variables|Default|GetHeldObject)
    (:Is%20Valid
      (if (> (Math|Vector|VectorLength _returnvalue_3) 3e+04)
        (Physics|AddForce _returnvalue_5 (* (Math|Vector|Normalize _returnvalue_3 0.01) 1.4e+04) "None" true)
        (Transformation|SetWorldRotation _returnvalue_5 (Math|Conversions|RotationFromXVector (Math|Vector|MakeVector (.x _returnvalue_7) (+ (.y _returnvalue_7) 1.8e+02) 0.0)) false false)))
    (:Is%20Not%20Valid
      (bind (_outhit _returnvalue_9) (Collision|LineTraceForObjects _returnvalue_8 (+ _returnvalue_8 (* (Math|Vector|GetForwardVector _returnvalue_4) (Variables|Default|GetPickupRange))) (Variables|Default|GetLineTraceableObjects) false 0 "None" true "(R=1.000000,G=0.000000,B=0.000000,A=1.000000)" "(R=0.000000,G=1.000000,B=0.000000,A=1.000000)" 2.0))
      (if _returnvalue_9
        (bind _aspickup (Utilities|Casting|CastToPickup (.HitActor (Collision|BreakHitResult _outhit)))
          (:then
            (Rendering|SetCustomDepthStencilValue (Variables|/Game/Blueprints/Pickup.Pickup_C|GetGeometry _aspickup) 1)
            (Utilities|IsValid (Variables|Default|GetLineTracedObject)
              (:Is%20Not%20Valid
                (Variables|Default|SetLineTracedObject _aspickup))))
          (:CastFailed
            (Utilities|IsValid (Variables|Default|GetLineTracedObject) :!label _label
              (:Is%20Valid
                (Rendering|SetCustomDepthStencilValue (Variables|/Game/Blueprints/Pickup.Pickup_C|GetGeometry (Variables|Default|GetLineTracedObject)) 0)
                (Variables|Default|SetLineTracedObject 0)))))
        (else
          (goto _label))))))