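; First-person player character that moves, looks, jumps, picks up objects, interacts and switches between time periods.
; Input delegates to PickupAgent, InteractAgent and TImeMachine components, with camera pitch clamped manually.
; A Transition timeline, exposed by getter and rate-scaled to WarpTime, is meant to feed fade curves into TImeMachine.
; Render-target preview code is unwired and marked broken, and IsInPresent returns IsInPast unnegated.
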(event EventBeginPlay
  (Components|Timeline|SetPlayRate (Variables|Default|GetTransition) (/ 1.0 (Variables|/Game/Blueprints/TImeMachine.TImeMachine_C|GetWarp%20Time (Variables|Default|GetTImeMachine)))))

(event Input|ActionEvents|InputActionJump
  (params (Key :type Key%20Structure))
  (:Pressed
    (Character|Jump)))

(event Input|ActionEvents|InputActionSwap
  (params (Key :type Key%20Structure))
  (:Pressed
    (Default|SwitchTime (Variables|Default|GetTImeMachine))
    (Default|OnTimeShifter (Variables|Default|GetPickupAgent))))

(event Input|AxisEvents|InputAxisVertical
  (params (AxisValue :type Float%20%28single-precision%29))
  (CallFunction|HandleInput AxisValue (stale Input|AxisEvents|InputAxisHorizontal AxisValue)))

(event Input|AxisEvents|InputAxisHorizontal
  (params (AxisValue :type Float%20%28single-precision%29))
  (CallFunction|HandleInput (stale Input|AxisEvents|InputAxisVertical AxisValue) AxisValue))

(event Input|MouseEvents|MouseX
  (params (AxisValue :type Float%20%28single-precision%29))
  (Pawn|Input|AddControllerYawInput AxisValue))

(event Input|MouseEvents|MouseY
  (params (AxisValue :type Float%20%28single-precision%29))
  (CallFunction|AddCameraPitchInput AxisValue))

(event Input|KeyboardEvents|E
  (params (Key :type Key%20Structure))
  (:Pressed
    (Default|CheckInteraction (Variables|Default|GetInteractAgent))))

(event Input|MouseEvents|LeftMouseButton
  (params (Key :type Key%20Structure))
  (:Pressed
    (Default|TogglePickup (Variables|Default|GetPickupAgent))))

(fn ConstructionScript)

(fn HandleInput
  (params (Vertical :type Float%20%28single-precision%29) (Horizontal :type Float%20%28single-precision%29))
  (bind _capsulecomponent (Variables|Collision|GetCapsuleComponent))
  (Class|PawnMovementComponent|AddInputVector (Variables|Character|GetCharacterMovement) (+ (* (Math|Vector|GetForwardVector _capsulecomponent) Vertical) (* (Math|Vector|GetRightVector _capsulecomponent) Horizontal)) false))

(fn AddCameraPitchInput
  (params (Value :type Float%20%28single-precision%29))
  (bind _camera (Variables|Default|GetCamera))
  (bind _relativerotation (Variables|/Script/Engine.SceneComponent|GetRelativeRotation _camera))
  (Transformation|AddRelativeRotation (Variables|Default|GetCamera) (Math|Rotator|MakeRotator 0.0 Value 0.0) false false)
  (if (< (.pitch _relativerotation) (CallFunction|-float (Variables|Default|GetCamera%20Max%20Angle)))
    (Transformation|SetRelativeRotation (Variables|Default|GetCamera) (Math|Rotator|MakeRotator 0.0 (CallFunction|-float (Variables|Default|GetCamera%20Max%20Angle)) 0.0) false false)
    (elif (> (.pitch _relativerotation) (Variables|Default|GetCamera%20Max%20Angle))
      (Transformation|SetRelativeRotation (Variables|Default|GetCamera) (Math|Rotator|MakeRotator 0.0 (Variables|Default|GetCamera%20Max%20Angle) 0.0) false false))))

(fn -float
  (params (value :type Float%20%28single-precision%29))
  (return (* value -1.0)))

(fn GetTransitionTimeline
  (return (Variables|Default|GetTransition)))

(fn IsinPresent
  (return (Variables|/Game/Blueprints/TImeMachine.TImeMachine_C|GetIs%20In%20Past (Variables|Default|GetTImeMachine))))