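; TreePast is an interactable tree for the past timeline that grows when given a Seed.
; An interaction outside the present with a held Seed and a valid LinkedObject destroys the seed.
; It then calls Set on the linked TreePresent, makes its own Tree component visible, and spawns a Key with a hardcoded ID at the Spawnbtheer actor's transform.
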(event EventOnInteract
  (params (Held%20Object :type Pickup%20Object%20Reference) (In%20Present :type Boolean))
  (bind _linkedobject (Variables|Default|GetLinkedObject))
  (if (not In%20Present)
    (Utilities|IsValid Held%20Object
      (:Is%20Valid
        (bind _asseed (Utilities|Casting|CastToSeed Held%20Object))
        (Utilities|IsValid _linkedobject
          (:Is%20Valid
            (Actor|DestroyActor _asseed)
            (bind _astree_present (Utilities|Casting|CastToTreePresent _linkedobject))
            (Default|Set _astree_present)
            (CallFunction|Set)
            (bind _returnvalue (Game|SpawnActorfromClass "/Game/Blueprints/Key.Key_C" (Transformation|GetActorTransform (Variables|Default|Getspawnbtheer)) "Undefined" 0 0))
            (Variables|/Game/Blueprints/Key.Key_C|SetkeyID _returnvalue 5)))))))

(fn ConstructionScript
  (|CallParentFunction))

(fn Set
  (Rendering|SetVisibility (Variables|Default|GetTree) true false))