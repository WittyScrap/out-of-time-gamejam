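; InteractAgent is a component that lets its owning player detect and interact with InteractableBase objects in view.
; Each tick it line-traces forward from the owner's camera, stores any interactable hit as SeenObject and shows or clears the CrosshairHUD prompt.
; CheckInteraction calls OnInteract on SeenObject, passing the PickupAgent's held object and the negation of the player's IsInPresent state as InPresent.
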(event EventBeginPlay)

(event EventTick
  (params (DeltaSeconds :type Float%20%28single-precision%29))
  (bind _returnvalue (Components|GetOwner))
  (bind _returnvalue_2 (Actor|GetComponentbyClass _returnvalue "/Script/Engine.CameraComponent"))
  (bind _returnvalue_3 (Transformation|GetWorldLocation _returnvalue_2))
  (bind (_outhit _returnvalue_4) (Collision|LineTraceForObjects _returnvalue_3 (+ _returnvalue_3 (* (Math|Vector|GetForwardVector _returnvalue_2) (Variables|Default|GetinteractionRange))) (Variables|Default|GetobjectTypes) false 0 "None" true "(R=1.000000,G=0.000000,B=0.000000,A=1.000000)" "(R=0.000000,G=1.000000,B=0.000000,A=1.000000)" 2.0))
  (if _returnvalue_4
    (bind _asinteractable_base (Utilities|Casting|CastToInteractableBase (.HitActor (Collision|BreakHitResult _outhit)))
      (:then
        (Variables|Default|SetseenObject _asinteractable_base)
        ;[0 1 0] HUD (press E to interact)
        (bind _ascrosshair_hud (Utilities|Casting|CastToCrosshairHUD (HUD|GetHUD (Game|GetPlayerController 0))))
        (Default|SetPromptText _ascrosshair_hud "[ E ] - Interact" -1.0))
      (:CastFailed
        (Variables|Default|SetseenObject 0 :!label _label)
        ;[0 1 0] HUD (clear prompts)
        (bind _ascrosshair_hud_2 (Utilities|Casting|CastToCrosshairHUD (HUD|GetHUD (Game|GetPlayerController 0))))
        (Default|SetPromptText _ascrosshair_hud_2 "" -1.0)))
    (else
      (goto _label))))

(fn CheckInteraction
  (bind _seenobject (Variables|Default|GetseenObject))
  (Utilities|IsValid _seenobject
    (:Is%20Valid
      (bind _asplayer (Utilities|Casting|CastToPlayer (Components|GetOwner)))
      (Default|OnInteract _seenobject (Variables|/Game/Blueprints/PickupAgent.PickupAgent_C|GetHeldObject (Actor|GetComponentbyClass (Components|GetOwner) "/Game/Blueprints/PickupAgent.PickupAgent_C")) (not (Default|IsinPresent _asplayer))))))