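; SafeScroller is an interactable number dial, apparently for a safe lock, that shows its current value as text.
; On interact, it increments CurrentStep and wraps back to zero once the value exceeds NumberOfSteps.
; It then writes the step number to its TextRender component.
; The construction script only calls the parent's.
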(event EventOnInteract
  (params (Held%20Object :type Pickup%20Object%20Reference) (In%20Present :type Boolean))
  (Utilities|FlowControl|Sequence
    (:then_0
      (Math|Integer|IncrementInt (Variables|Default|Getcurrent_step)
        (:%20%20
          (if (> (Variables|Default|Getcurrent_step) (Variables|Default|Getnumber_of_steps))
            (Variables|Default|Setcurrent_step 0)))))
    (:then_1
      (Rendering|Components|TextRender|SetText (Variables|Default|GetTextRender) (Utilities|Text|ToText(Integer) (Variables|Default|Getcurrent_step) false true 1 1)))))

(fn ConstructionScript
  (|CallParentFunction))