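; Interactable safe Blueprint that checks a combination lock when the player interacts with it.
; It compares each scroller's current step against the matching entry in an array of correct values, stopping at the first mismatch.
; The result sets a SafeOpened flag and shows a timed success or failure prompt on the crosshair HUD.
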(event EventOnInteract
  (params (Held%20Object :type Pickup%20Object%20Reference) (In%20Present :type Boolean))
  (bind _returnvalue (Game|GetPlayerController 0))
  (bind _returnvalue_2 (HUD|GetHUD _returnvalue))
  (Variables|Default|Setsafe_opened true)
  (bind _index (Utilities|FlowControl|ForLoopwithBreak 0 (- (Utilities|Array|Length (Variables|Default|Getscrollers)) 1) :!label _label)
    (:LoopBody
      (if (not (== (Variables|/Game/Blueprints/SafeScroller.SafeScroller_C|Getcurrent_step (Utilities|Array|Get(acopy) (Variables|Default|Getscrollers) _index)) (Utilities|Array|Get(acopy) (Variables|Default|Getcorrect_values) _index)))
        (Variables|Default|Setsafe_opened false)
        (goto _label Break)))
    (:Completed
      (if (Variables|Default|Getsafe_opened)
        ;[1 1 1] SAFE OPENED
        (bind _ascrosshair_hud (Utilities|Casting|CastToCrosshairHUD _returnvalue_2))
        (Default|SetPromptText _ascrosshair_hud "Safe opened" 2.0)
        (else
          ;[1 1 1] SAFE OPEN FAILED
          (bind _ascrosshair_hud_2 (Utilities|Casting|CastToCrosshairHUD _returnvalue_2))
          (Default|SetPromptText _ascrosshair_hud_2 "Safe is fucked" 2.0))))))

(fn ConstructionScript
  (|CallParentFunction))