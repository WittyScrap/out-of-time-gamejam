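; Actor component that lets the player jump between past and present versions of the level, stacked vertically by a fixed height.
; Switching flips the past flag, plays the Player's transition and, halfway through the warp time, teleports the owner up or down by that height.
; A camera update mirrors a source camera's transform into the other era with that offset.
; An animation function lerps the owner camera's FOV toward a target.
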(event Custom|Do%20Warp
  (Utilities|FlowControl|Delay (/ (Variables|Default|GetWarp%20Time) 2.0))
  (CallFunction|PerformWarp))

(event EventBeginPlay
  (Variables|Default|SetFOV%20Start (Variables|/Script/Engine.CameraComponent|GetFieldOfView (Actor|GetComponentbyClass (Components|GetOwner) "/Script/Engine.CameraComponent"))))

(fn SwitchTime
  (Utilities|FlowControl|Sequence
    (:then_0
      (if (Variables|Default|GetIs%20In%20Past)
        (Variables|Default|SetDirection 1.0)
        (else
          (Variables|Default|SetDirection -1.0))))
    (:then_2
      (Variables|Default|SetIs%20In%20Past (not (Variables|Default|GetIs%20In%20Past)))
      (bind _asplayer (Utilities|Casting|CastToPlayer (Components|GetOwner)))
      (Components|Timeline|PlayfromStart (Variables|/Game/Blueprints/Player.Player_C|GetTransition _asplayer))
      (CallFunction|DoWarp))))

(fn UpdateCamera
  (params (Target%20Camera :type Scene%20Capture%20Component%202D%20Object%20Reference%20%28by%20ref%29) (Source%20Camera :type Camera%20Component%20Object%20Reference%20%28by%20ref%29))
  (bind _returnvalue (Transformation|GetWorldLocation Source%20Camera))
  (bind _returnvalue_2 (Transformation|GetWorldLocation Source%20Camera))
  (Utilities|FlowControl|Sequence
    (:then_0
      (if (Variables|Default|GetIs%20In%20Past)
        (Transformation|SetWorldLocation Target%20Camera (Math|Vector|MakeVector (.x _returnvalue_2) (.y _returnvalue_2) (+ (.z _returnvalue_2) (Variables|Default|GetSwitch%20Height))) false true)
        (else
          (Transformation|SetWorldLocation Target%20Camera (Math|Vector|MakeVector (.x _returnvalue) (.y _returnvalue) (- (.z _returnvalue) (Variables|Default|GetSwitch%20Height))) false true))))
    (:then_1
      (Transformation|SetWorldRotation Target%20Camera (Transformation|GetWorldRotation Source%20Camera) false false))))

(fn RunAnimation
  (params (Linear :type Float%20%28single-precision%29) (Exponential :type Float%20%28single-precision%29))
  (Camera|SetFieldOfView (Actor|GetComponentbyClass (Components|GetOwner) "/Script/Engine.CameraComponent") (Math|Float|Lerp (Variables|Default|GetFOV%20Start) (Variables|Default|GetFOV%20Target) Exponential)))

(fn PerformWarp
  (Transformation|AddActorWorldOffset (Components|GetOwner) (Math|Vector|MakeVector 0.0 0.0 (* (Variables|Default|GetSwitch%20Height) (Variables|Default|GetDirection))) false true))