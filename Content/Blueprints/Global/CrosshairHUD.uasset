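; HUD Blueprint that draws a screen-centered crosshair and a text prompt along the bottom edge.
; DrawHUD draws four diagonal ticks with a gap in the middle, then centers the prompt horizontally using its measured size.
; SetPromptText sets the text, and a non-negative time starts a Delay in CheckDelay that clears it.
; Calls during a running Delay do not restart it, so the pending clear still fires.
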(event Custom|Check%20Delay
  (Utilities|FlowControl|Delay (Variables|Default|GetReset%20Delay))
  (Variables|Default|SetReset%20Delay 0.0)
  (CallFunction|SetPromptText "" -1.0))

(event EventDrawHUD
  (params (SizeX :type Integer) (SizeY :type Integer))
  (CallFunction|DrawFancyCrosshair SizeX SizeY)
  (CallFunction|DrawPromptText (Math|Conversions|ToFloat(Integer) SizeX) (Math|Conversions|ToFloat(Integer) SizeY)))

(fn ConstructionScript)

(fn DrawFancyCrosshair
  (params (Size%20X :type Integer) (Size%20Y :type Integer))
  (bind _returnvalue (/ Size%20Y 2))
  (bind _returnvalue_2 (/ Size%20X 2))
  (bind _returnvalue_3 (Math|Conversions|ToFloat(Integer) _returnvalue))
  (bind _returnvalue_4 (Math|Conversions|ToFloat(Integer) _returnvalue_2))
  (bind _returnvalue_5 (+ _returnvalue_4 -5.0))
  (bind _returnvalue_6 (+ _returnvalue_3 5.0))
  (bind _returnvalue_7 (+ _returnvalue_3 -5.0))
  (bind _returnvalue_8 (+ _returnvalue_4 5.0))
  (bind _returnvalue_9 (+ _returnvalue_3 1e+01))
  (bind _returnvalue_10 (+ _returnvalue_3 -1e+01))
  (bind _returnvalue_11 (+ _returnvalue_4 1e+01))
  (bind _returnvalue_12 (+ _returnvalue_4 -1e+01))
  (Class|HUD|DrawLine _returnvalue_12 _returnvalue_9 _returnvalue_5 _returnvalue_6 "(R=1.000000,G=1.000000,B=1.000000,A=1.000000)" 1.0) ; Left Up
  (Class|HUD|DrawLine _returnvalue_12 _returnvalue_10 _returnvalue_5 _returnvalue_7 "(R=1.000000,G=1.000000,B=1.000000,A=1.000000)" 1.0) ; Left Down
  (Class|HUD|DrawLine _returnvalue_11 _returnvalue_9 _returnvalue_8 _returnvalue_6 "(R=1.000000,G=1.000000,B=1.000000,A=1.000000)" 1.0) ; Right Up
  (Class|HUD|DrawLine _returnvalue_11 _returnvalue_10 _returnvalue_8 _returnvalue_7 "(R=1.000000,G=1.000000,B=1.000000,A=1.000000)" 1.0) ; Right Down
)

(fn DrawPromptText
  (params (Screen%20Width :type Float%20%28single-precision%29) (Screen%20Height :type Float%20%28single-precision%29))
  (bind _prompt_text_font (Variables|Default|GetPrompt%20Text%20Font))
  (bind _prompt_text (Variables|Default|GetPrompt%20Text))
  (bind _prompt_text_scale (Variables|Default|GetPrompt%20Text%20Scale))
  (bind (_outwidth _outheight) (Class|HUD|GetTextSize _prompt_text _prompt_text_font _prompt_text_scale))
  (HUD|DrawText (Variables|Default|GetPrompt%20Text) "(R=1.000000,G=1.000000,B=1.000000,A=1.000000)" (|((width/2)-(textWidth/2)) Screen%20Width _outwidth) (- Screen%20Height _outheight) (Variables|Default|GetPrompt%20Text%20Font) (Variables|Default|GetPrompt%20Text%20Scale) false))

(fn SetPromptText
  (params (Value :type String) (Time :type Float%20%28single-precision%29))
  (Variables|Default|SetPrompt%20Text Value)
  (if (>= Time 0.0)
    (CallFunction|SetResetDelay Time)))

(fn SetResetDelay
  (params (Amount :type Float%20%28single-precision%29))
  (Variables|Default|SetReset%20Delay Amount)
  (CallFunction|CheckDelay))