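; Interactable double door that opens and closes with sound and can be locked until a held Key with a matching ID is used.
; A matching key unlocks it and its linked Door without opening them, while other attempts play a locked animation.
; Timelines drive RotateDoors, which yaws both leaves in opposite directions.
; Toggling calls ForcedInteraction on LinkedObject, where a linked Door unlocks and toggles only if its state differs, ending the mutual callback.
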(event EventForcedInteraction
  (params (sender :type Interactable%20Base%20Object%20Reference))
  (bind _returnvalue (Transformation|GetActorLocation))
  (bind _linkedobject (Variables|Default|GetLinkedObject))
  (bind _asdoor (Utilities|Casting|CastToDoor sender))
  (Variables|Default|SetisLocked false)
  (if (Math|Boolean|NotEqual(Boolean) (Variables|Door_C|GetisOpen _asdoor) (Variables|Default|GetisOpen))
    (bind _output_get (Variables|Default|SetisOpen (not (Variables|Default|GetisOpen))))
    (Utilities|FlowControl|Sequence
      (:then_0
        (if _output_get
          (Audio|PlaySoundatLocation "/Engine/VREditor/Sounds/UI/Laser_Push.Laser_Push" _returnvalue "0, 0, 0" 1.0 1.0 0.0 0 0 0)
          (bind _rotation (Timeline|DoorAnimation Play)
            (:Update
              (CallFunction|RotateDoors _rotation)))
          (else
            (Audio|PlaySoundatLocation "/Engine/VREditor/Sounds/UI/Laser_Push.Laser_Push" _returnvalue "0, 0, 0" 1.0 1.0 0.0 0 0 0)
            (Timeline|DoorAnimation Reverse))))
      (:then_1
        (Utilities|IsValid _linkedobject
          (:Is%20Valid
            (Default|ForcedInteraction _linkedobject self)))))))

(event EventOnInteract
  (params (Held%20Object :type Pickup%20Object%20Reference) (In%20Present :type Boolean))
  (bind _returnvalue (Transformation|GetActorLocation))
  (bind _linkedobject (Variables|Default|GetLinkedObject))
  (if (Variables|Default|GetisLocked)
    (Utilities|IsValid Held%20Object
      (:Is%20Valid
        (bind _askey (Utilities|Casting|CastToKey Held%20Object)
          (:then
            (if (== (Variables|Default|GetkeyHoleID) (Variables|/Game/Blueprints/Key.Key_C|GetkeyID _askey))
              (Variables|Default|SetisLocked false)
              (bind _asdoor (Utilities|Casting|CastToDoor (Variables|Default|GetLinkedObject)))
              (Variables|Door_C|SetisLocked _asdoor false)
              (else
                (bind _rotate (Timeline|LockedDoorAnimation PlayFromStart)
                  (:Update
                    (CallFunction|RotateDoors _rotate))))))
          (:CastFailed
            (Timeline|LockedDoorAnimation PlayFromStart))))
      (:Is%20Not%20Valid
        (Timeline|LockedDoorAnimation PlayFromStart)))
    (else
      (bind _output_get (Variables|Default|SetisOpen (not (Variables|Default|GetisOpen))))
      (Utilities|FlowControl|Sequence
        (:then_0
          (if _output_get
            (Audio|PlaySoundatLocation "/Engine/VREditor/Sounds/UI/Laser_Push.Laser_Push" _returnvalue "0, 0, 0" 1.0 1.0 0.0 0 0 0)
            (bind _rotation (Timeline|DoorAnimation Play)
              (:Update
                (CallFunction|RotateDoors _rotation)))
            (else
              (Audio|PlaySoundatLocation "/Engine/VREditor/Sounds/UI/Laser_Push.Laser_Push" _returnvalue "0, 0, 0" 1.0 1.0 0.0 0 0 0)
              (Timeline|DoorAnimation Reverse))))
        (:then_1
          (Utilities|IsValid _linkedobject
            (:Is%20Valid
              (Default|ForcedInteraction _linkedobject self))))))))

(fn ConstructionScript
  (|CallParentFunction))

(fn RotateDoors
  (params (Angle :type Float%20%28single-precision%29))
  (Transformation|SetRelativeRotation (Variables|Default|GetLeft%20Door) (Math|Rotator|MakeRotator 0.0 0.0 Angle) false false)
  (Transformation|SetRelativeRotation (Variables|Default|GetRight%20Door) (Math|Rotator|MakeRotator 0.0 0.0 (* Angle -1.0)) false false))